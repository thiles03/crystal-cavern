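; BP_WinVolume is a trigger volume that ends a level when the player overlaps it after collecting every crystal.
; On overlap it checks that no BP_Crystal actors remain, then once fades the camera to black and waits briefly.
; It finds the current level in a LevelNames array and opens the next entry, doing nothing more on the final level.
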(event Collision|EventActorBeginOverlap
  (params (OtherActor :type Actor%20Object%20Reference))
  (Utilities|IsPlayer OtherActor
    (:IsPlayer
      (if (not (CallFunction|AnyCrystalsRemaining))
        (Utilities|FlowControl|DoOnce false
          (:Completed
            (CameraFades|StartCameraFade :self (Game|GetPlayerCameraManager 0) :ToAlpha 1.0 :Duration 2.0 :bHoldWhenFinished true)
            (Utilities|FlowControl|Delay 3.0)
            (LevelManagement|CompleteLevel)))))))

(fn ConstructionScript)

(fn AnyCrystalsRemaining
  (bind _outactors (Actor|GetAllActorsOfClass "/Game/Blueprints/Actors/Collectibles/BP_Crystal.BP_Crystal_C"))
  (return (> (Utilities|Array|Length _outactors) 0)))

(fn CompleteLevel
  (if (not (LevelManagement|IsFinalLevel))
    (LevelManagement|LoadNextLevel)))

(fn GetCurrentLevelIndex
  (bind _returnvalue (Game|GetCurrentLevelName true))
  (return (Utilities|Array|FindItem (Variables|Default|GetLevelNames) (Utilities|String|StringToName _returnvalue))))

(fn IsFinalLevel
  (return (== (Utilities|Array|LastIndex (Variables|Default|GetLevelNames)) (LevelManagement|GetCurrentLevelIndex))))

(fn LoadNextLevel
  (Game|OpenLevel(byName) (LevelManagement|GetNextLevelName)))

(fn GetNextLevelName
  (return (Utilities|Array|Get(acopy) (Variables|Default|GetLevelNames) (+ (LevelManagement|GetCurrentLevelIndex) 1))))