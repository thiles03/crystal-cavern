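; Collectible crystal actor that spins around its yaw axis and is absorbed by the player on overlap.
; On player overlap it caches its location, scale and point light intensity, then plays a timeline.
; The timeline's progress lerps it toward the player pawn's current position while shrinking it and fading its light, then the actor is destroyed.
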(event EventTick
  (params (DeltaSeconds :type Float%20%28single-precision%29))
  ;[1 1 1] Rotate
  (Transformation|AddActorLocalRotation (Math|Rotator|MakeRotator 0.0 0.0 (Variables|Default|GetRotationSpeed)) false false))

(event Collision|EventActorBeginOverlap
  (params (OtherActor :type Actor%20Object%20Reference))
  ;[1 1 1] Collect and destroy
  (Utilities|IsPlayer OtherActor
    (:IsPlayer
      (CallFunction|StoreStartValues)
      (bind _collectionprogress (Timeline|CollectionTimeline Play)
        (:Update
          (CallFunction|ShrinktoPlayer _collectionprogress _collectionprogress _collectionprogress))
        (:Finished
          (Actor|DestroyActor))))))

(fn ConstructionScript)

(fn MovetoPlayer
  (params (Alpha :type Float%20%28single-precision%29))
  (Transformation|SetActorLocation (Math|Vector|Lerp(Vector) (Variables|Default|GetStartLocation) (Transformation|GetActorLocation (Game|Player|GetPlayerPawn 0)) Alpha) false false))

(fn StoreStartValues
  (Variables|Default|SetStartLocation (Transformation|GetActorLocation))
  (Variables|Default|SetStartScale (Transformation|GetActorScale3D))
  (Variables|Default|SetStartLightIntensity (Variables|/Script/Engine.LightComponentBase|GetIntensity (Variables|Default|GetPointLight))))

(fn ScaletoZero
  (params (Alpha :type Float%20%28single-precision%29))
  (Transformation|SetActorScale3D (Math|Vector|Lerp(Vector) (Variables|Default|GetStartScale) "0, 0, 0" Alpha)))

(fn DecreaseLightIntensity
  (params (Alpha :type Float%20%28single-precision%29))
  (Rendering|Components|Light|SetIntensity (Variables|Default|GetPointLight) (Math|Float|Lerp (Variables|Default|GetStartLightIntensity) 0.0 Alpha)))

(fn ShrinktoPlayer
  (params (MoveTime :type Float%20%28single-precision%29) (ScaleTime :type Float%20%28single-precision%29) (FadeTime :type Float%20%28single-precision%29))
  (CallFunction|MovetoPlayer MoveTime)
  (CallFunction|ScaletoZero ScaleTime)
  (CallFunction|DecreaseLightIntensity FadeTime))