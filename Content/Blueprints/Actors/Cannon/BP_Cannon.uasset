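; BP_Cannon is a cannon actor that automatically fires BP_Projectile on a repeating cycle from the start of play.
; After a FireRate delay, it spawns a projectile at ProjectileSpawnPoint's location and rotation, scaled by ProjectileScale.
; A timeline then slides the barrel along its relative Y axis to animate the shot.
; The timeline's Cannon Fired event track loops back to the delay, sustaining the cycle without Tick.
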(event EventBeginPlay
  (Utilities|FlowControl|Delay (Variables|CannonProperties|GetFireRate) :!label _label)
  (CallFunction|SpawnProjectile)
  (bind _barrellocation (Timeline|CannonFireTimeline PlayFromStart)
    (:Update
      (CallFunction|MoveCannonBarrel _barrellocation))
    (:CannonFired
      (goto _label))))

(event Collision|EventActorBeginOverlap
  (params (OtherActor :type Actor%20Object%20Reference)))

(event EventTick
  (params (DeltaSeconds :type Float%20%28single-precision%29)))

(fn ConstructionScript)

(fn SpawnProjectile
  (bind _projectilespawnpoint (Variables|Default|GetProjectileSpawnPoint))
  (Game|SpawnActorfromClass "/Game/Blueprints/Actors/Projectiles/BP_Projectile.BP_Projectile_C" (Math|Transform|MakeTransform (Transformation|GetWorldLocation _projectilespawnpoint) (Transformation|GetWorldRotation _projectilespawnpoint) (Math|Conversions|ToVector(Float) (Variables|CannonProperties|GetProjectileScale))) "AlwaysSpawn" 0 0))

(fn MoveCannonBarrel
  (params (CannonBarrelYLocation :type Float%20%28single-precision%29))
  (Transformation|SetRelativeLocation (Variables|Default|GetBarrel) (Math|Vector|MakeVector 0.0 CannonBarrelYLocation 0.0) false false))